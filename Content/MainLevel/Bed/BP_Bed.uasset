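; BP_Bed is a clickable bed that puts the player to sleep and resets the main level's daily state, unless BP_FleshPit is eating.
; Clicking clears MainCharacter's market, harvest and paperboy flags, restores garden and potion shop sprites, rolls and shows a new BP_PaperBoy visitor, and hides BP_TimmyJS.
; A snore and timed camera fade cover the transition, with click events disabled and both HUD widgets removed, then recreated afterwards.
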(event `self.PaperSprite.OnClicked`
  (params (TouchedComponent :type "PrimitiveComponent Object Reference") (ButtonPressed :type "Key Structure"))
  (bind _returnvalue (`GameplayStatics.GetPlayerCameraManager` 0))
  (bind _returnvalue_2 (`GameplayStatics.GetActorOfClass` "/Game/MainLevel/FleshPit/BP_FleshPit.BP_FleshPit_C"))
  (if (not (`/Game/MainLevel/FleshPit/BP_FleshPit.Eating` _returnvalue_2))
    (bind _asmain_character (cast `/Game/Character/MainCharacter` (`GameplayStatics.GetPlayerPawn` 0)))
    (set `PlayerController.bEnableClickEvents` false (`GameplayStatics.GetPlayerController` 0))
    (bind _foundwidgets (`WidgetBlueprintLibrary.GetAllWidgetsOfClass` "/Game/Character/CharacterUI.CharacterUI_C"))
    (`Widget.RemoveFromParent` _foundwidgets)
    (bind _foundwidgets_2 (`WidgetBlueprintLibrary.GetAllWidgetsOfClass` "/Game/Character/WB_Stats.WB_Stats_C"))
    (`Widget.RemoveFromParent` _foundwidgets_2)
    (`KismetSystemLibrary.PrintString` "sleep time")
    (`GameplayStatics.PlaySound2D` "/Game/MainLevel/Bed/Snore.Snore" 0.5 1.0 0.0 null null)
    (set `/Game/Character/MainCharacter.WentToMarket` false _asmain_character)
    (set `/Game/Character/MainCharacter.HasHarvested` false _asmain_character)
    (set `/Game/Character/MainCharacter.PaperBoyVisited` false _asmain_character)
    (bind _returnvalue_3 (`GameplayStatics.GetActorOfClass` "/Game/MainLevel/Garden/BP_Garden.BP_Garden_C"))
    (`PaperSpriteComponent.SetSprite` (`/Game/MainLevel/Garden/BP_Garden.PaperSprite` _returnvalue_3) "/Game/MainLevel/Garden/Sprites/New_Piskel__11___2__Sprite_1.New_Piskel__11___2__Sprite_1")
    (bind _returnvalue_4 (`GameplayStatics.GetActorOfClass` "/Game/MainLevel/PotionShop/BP_PotionShop.BP_PotionShop_C"))
    (`PaperSpriteComponent.SetSprite` (`/Game/MainLevel/PotionShop/BP_PotionShop.PaperSprite` _returnvalue_4) "/Game/MainLevel/PotionShop/New_Piskel__11___3__Sprite1.New_Piskel__11___3__Sprite1")
    (bind _returnvalue_5 (`GameplayStatics.GetActorOfClass` "/Game/MainLevel/PaperBoy/BP_PaperBoy.BP_PaperBoy_C"))
    (set `/Game/MainLevel/PaperBoy/BP_PaperBoy.Visitor` (`KismetMathLibrary.RandomIntegerInRange` (`self.Who`) (`self.Visits`)) _returnvalue_5)
    (`/Game/MainLevel/PaperBoy/BP_PaperBoy.SetVisitor` _returnvalue_5)
    (`self.SetActorHiddenInGame` _returnvalue_5 false)
    (`PrimitiveComponent.SetCollisionEnabled` (`/Game/MainLevel/PaperBoy/BP_PaperBoy.PaperSprite` _returnvalue_5) "QueryAndPhysics")
    (bind _returnvalue_6 (`GameplayStatics.GetActorOfClass` "/Game/MainLevel/PaperBoy/Sprites/Closeup/TiimyJumpscare/BP_TimmyJS.BP_TimmyJS_C"))
    (`self.SetActorHiddenInGame` _returnvalue_6 true)
    (`PlayerCameraManager.StartCameraFade` :`self` _returnvalue :`ToAlpha` 1.0 :`Duration` 1.0 :`bHoldWhenFinished` true)
    (`KismetSystemLibrary.Delay` 1.5)
    (`PlayerCameraManager.StartCameraFade` :`self` _returnvalue :`FromAlpha` 1.0 :`Duration` 1.0)
    (`KismetSystemLibrary.Delay` 1.0)
    (set `PlayerController.bEnableClickEvents` true (`GameplayStatics.GetPlayerController` 0))
    (bind _returnvalue_7 (`|CreateWidget` "/Game/Character/CharacterUI.CharacterUI_C"))
    (bind _returnvalue_8 (`|CreateWidget` "/Game/Character/WB_Stats.WB_Stats_C"))
    (`UserWidget.AddToViewport` _returnvalue_8 0)
    (`UserWidget.AddToViewport` _returnvalue_7 0)))

(fn `UserConstructionScript`)