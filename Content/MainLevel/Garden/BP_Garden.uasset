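; BP_Garden is a clickable garden that gives the player food units when harvested.
; Clicking its Paper2D sprite checks the MainCharacter's HasHarvested flag, playing a refusal or harvest sound with debug prints.
; A harvest adds FarmUpgrade times a random yield to CurrentFoodUnits, sets the flag and swaps the sprite.
; The random node is pure, so the printed yield can differ from the amount added.
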(event `self.PaperSprite.OnClicked`
  (params (TouchedComponent :type "PrimitiveComponent Object Reference") (ButtonPressed :type "Key Structure"))
  (bind _asmain_character (cast `/Game/Character/MainCharacter` (`GameplayStatics.GetPlayerPawn` 0)))
  (if (`/Game/Character/MainCharacter.HasHarvested` _asmain_character)
    (`KismetSystemLibrary.PrintString` "No more to harvest")
    (`GameplayStatics.PlaySound2D` "/Game/MainLevel/Garden/477390__nuff3__steps-dirt_2a.477390__nuff3__steps-dirt_2a" 1.0 1.0 0.0 null null)
    (else
      (`KismetSystemLibrary.PrintString` "Just harvested")
      (`GameplayStatics.PlaySound2D` "/Game/MainLevel/Garden/699492__valenspire__plant_harvest_03.699492__valenspire__plant_harvest_03" 2.0 1.0 0.0 null null)
      (bind _returnvalue (* (`/Game/Character/MainCharacter.FarmUpgrade` _asmain_character) (`KismetMathLibrary.RandomIntegerInRange` (`self.DefaultMin`) (`self.DefaultMax`))))
      (`KismetSystemLibrary.PrintString` (`KismetStringLibrary.Conv_IntToString` _returnvalue))
      (bind _output_get (set `/Game/Character/MainCharacter.CurrentFoodUnits` (+ _returnvalue (`/Game/Character/MainCharacter.CurrentFoodUnits` _asmain_character)) _asmain_character))
      (`KismetSystemLibrary.PrintString` (`KismetStringLibrary.Conv_IntToString` _output_get))
      (set `/Game/Character/MainCharacter.HasHarvested` true _asmain_character)
      (`PaperSpriteComponent.SetSprite` (`self.PaperSprite`) "/Game/MainLevel/Garden/Sprites/New_Piskel__11___2__Sprite_0.New_Piskel__11___2__Sprite_0"))))

(fn `UserConstructionScript`)