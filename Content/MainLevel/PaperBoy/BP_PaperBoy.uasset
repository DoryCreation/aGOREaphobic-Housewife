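; Clickable visitor actor that appears as Timmy the paperboy, the neighbour, or a policeman if the neighbour is dead.
; SetVisitor picks the flipbook from Visitor and NeighbourDead.
; Clicking swaps CharacterUI widgets for that visitor's dialogue, hides the actor and plays a sound; Timmy also rolls a food offer and cost scaled by FarmUpgrade.
; A leftover E-key test messages BPI_Neighbour implementers, but its loop has no array input.
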(event `SetVisitor`
  (if (== (`self.Visitor`) 1)
    (if (`self.NeighbourDead`)
      (`PaperFlipbookComponent.SetFlipbook` (`self.FB_TimmyIdle`) "/Game/MainLevel/PaperBoy/Sprites/overworld/PoliceMan/FB_PoliceMan.FB_PoliceMan")
      (else
        (`PaperFlipbookComponent.SetFlipbook` (`self.FB_TimmyIdle`) "/Game/MainLevel/PaperBoy/Sprites/overworld/Neighbour/FB_NeignbourIdle.FB_NeignbourIdle")))
    (else
      (`PaperFlipbookComponent.SetFlipbook` (`self.FB_TimmyIdle`) "/Game/MainLevel/PaperBoy/Sprites/overworld/Timmy/FB_TimmyIdle.FB_TimmyIdle"))))

(event `self.PaperSprite.OnClicked`
  (params (TouchedComponent :type "PrimitiveComponent Object Reference") (ButtonPressed :type "Key Structure"))
  (`KismetSystemLibrary.PrintString` "Hello")
  (bind _asmain_character (cast `/Game/Character/MainCharacter` (`GameplayStatics.GetPlayerPawn` 0)))
  (if (== (`self.Visitor`) 1)
    (if (`self.NeighbourDead`)
      (bind _foundwidgets (`WidgetBlueprintLibrary.GetAllWidgetsOfClass` "/Game/Character/CharacterUI.CharacterUI_C"))
      (`Widget.RemoveFromParent` _foundwidgets)
      (bind _returnvalue (`|CreateWidget` "/Game/MainLevel/PaperBoy/WB_Police.WB_Police_C"))
      (`UserWidget.AddToViewport` _returnvalue 0)
      (`PrimitiveComponent.SetCollisionEnabled` (`self.PaperSprite`) "NoCollision")
      (`self.SetActorHiddenInGame` true)
      (`GameplayStatics.PlaySound2D` "/Game/MainLevel/PaperBoy/PoliceMan.PoliceMan" 0.25 1.0 0.0 null null)
      (else
        (bind _foundwidgets_2 (`WidgetBlueprintLibrary.GetAllWidgetsOfClass` "/Game/Character/CharacterUI.CharacterUI_C"))
        (`Widget.RemoveFromParent` _foundwidgets_2)
        (bind _returnvalue_2 (`|CreateWidget` "/Game/MainLevel/PaperBoy/WB_Neighnour.WB_Neighnour_C"))
        (`UserWidget.AddToViewport` _returnvalue_2 0)
        (`PrimitiveComponent.SetCollisionEnabled` (`self.PaperSprite`) "NoCollision")
        (`self.SetActorHiddenInGame` true)
        (`GameplayStatics.PlaySound2D` "/Game/MainLevel/PaperBoy/onlymp3_to_-_Stop_You_ve_violated_the_law_-My0lzMuNcHI-192k-1700437366.onlymp3_to_-_Stop_You_ve_violated_the_law_-My0lzMuNcHI-192k-1700437366" 0.25 1.0 0.0 null null)))
    (else
      (bind _foundwidgets_3 (`WidgetBlueprintLibrary.GetAllWidgetsOfClass` "/Game/Character/CharacterUI.CharacterUI_C"))
      (`Widget.RemoveFromParent` _foundwidgets_3)
      (bind _returnvalue_3 (`|CreateWidget` "/Game/MainLevel/PaperBoy/WP_Timmy.WP_Timmy_C"))
      (`UserWidget.AddToViewport` _returnvalue_3 0)
      (`PrimitiveComponent.SetCollisionEnabled` (`self.PaperSprite`) "NoCollision")
      (bind _farmupgrade (`/Game/Character/MainCharacter.FarmUpgrade` _asmain_character))
      (set `self.FoodOffer` (* (`KismetMathLibrary.RandomIntegerInRange` (`self.DefaultMin`) (`self.DefaultMax`)) _farmupgrade))
      (set `self.PaperBoyCost` (* (`self.BaseCost`) _farmupgrade))
      (`self.SetActorHiddenInGame` true)
      (`GameplayStatics.PlaySound2D` "/Game/MainLevel/PaperBoy/Hello.Hello" 0.25 1.0 0.0 null null))))

(event `Key|E`
  (params (Key :type "Key Structure"))
  ;[1 1 1] ollie fucking around
  (:`Pressed`
    (for _array_element _
      (if (`KismetSystemLibrary.DoesImplementInterface` _array_element "/Game/MainLevel/Dialogues/BPI_Neighbour.BPI_Neighbour_C")
        (message `/Game/MainLevel/Dialogues/BPI_Neighbour.NeighbourTalk` _array_element)))))

(fn `UserConstructionScript`)