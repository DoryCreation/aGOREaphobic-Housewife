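; BP_PotionShop is a clickable paper sprite shop where the player sells potions for money.
; On click it reads the main character pawn, and if the player has not yet been to market and holds potions, it adds potion value times count to Money.
; It then plays a coin sound, empties the potion count and sets WentToMarket to block further sales, with debug prints reporting each outcome.
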(event `self.PaperSprite.OnClicked`
  (params (TouchedComponent :type "PrimitiveComponent Object Reference") (ButtonPressed :type "Key Structure"))
  (bind _asmain_character (cast `/Game/Character/MainCharacter` (`GameplayStatics.GetPlayerPawn` 0)))
  (if (`/Game/Character/MainCharacter.WentToMarket` _asmain_character)
    (`KismetSystemLibrary.PrintString` "Went to Market Today Already")
    (elif (> (`/Game/Character/MainCharacter.CurrentPotionCount` _asmain_character) 0)
      (`KismetSystemLibrary.PrintString` "Got Potions")
      (`GameplayStatics.PlaySound2D` "/Game/MainLevel/PotionShop/360739__matrixxx__coin-sound-01.360739__matrixxx__coin-sound-01" 1.0 1.0 0.0 null null)
      (bind _output_get (set `/Game/Character/MainCharacter.Money` (+ (`/Game/Character/MainCharacter.Money` _asmain_character) (* (`self.PotionValue`) (`/Game/Character/MainCharacter.CurrentPotionCount` _asmain_character))) _asmain_character))
      (set `/Game/Character/MainCharacter.CurrentPotionCount` 0 _asmain_character)
      (`KismetSystemLibrary.PrintString` (`KismetStringLibrary.Conv_IntToString` _output_get))
      (set `/Game/Character/MainCharacter.WentToMarket` true _asmain_character)
      (else
        (`KismetSystemLibrary.PrintString` "No Potions")))))

(fn `UserConstructionScript`)