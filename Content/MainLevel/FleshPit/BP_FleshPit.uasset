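; BP_FleshPit is a clickable flesh pit that turns the player's food into potions.
; A click checks MainCharacter's digesting flag, food units, potion capacity and the pit's stomach limit.
; Success spends food, plays a one-second eating phase, then adds a potion, while any failed check plays a sound and a brief sad state.
; Tick switches the eat, sad or idle flipbook from the Eating and Sad flags.
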(event `self.ReceiveTick`
  (params (DeltaSeconds :type "Float (single-precision)"))
  (if (`self.Eating`)
    (`PaperFlipbookComponent.SetFlipbook` (`self.FB_Eat`) "/Game/MainLevel/FleshPit/Animations/Eating/FB_Eat.FB_Eat")
    (elif (`self.Sad`)
      (`PaperFlipbookComponent.SetFlipbook` (`self.FB_Eat`) "/Game/MainLevel/FleshPit/Animations/disagree/FB_Sad.FB_Sad")
      (else
        (`PaperFlipbookComponent.SetFlipbook` (`self.FB_Eat`) "/Game/MainLevel/FleshPit/Animations/Eating/FB_Idle.FB_Idle")))))

(event `self.PaperSprite.OnClicked`
  (params (TouchedComponent :type "PrimitiveComponent Object Reference") (ButtonPressed :type "Key Structure"))
  (bind _asmain_character (cast `/Game/Character/MainCharacter` (`GameplayStatics.GetPlayerPawn` 0)))
  (if (`/Game/Character/MainCharacter.PitIsDigesting` _asmain_character)
    (`KismetSystemLibrary.PrintString` "Has Been feed today already")
    (`GameplayStatics.PlaySound2D` "/Game/MainLevel/FleshPit/WAV_CurrentlyEating.WAV_CurrentlyEating" 1.0 1.0 0.0 null null :!label _label)
    (set `self.Sad` true)
    (`KismetSystemLibrary.Delay` 1.0)
    (set `self.Sad` false)
    (elif (>= (`/Game/Character/MainCharacter.CurrentFoodUnits` _asmain_character) (`self.FoodReqired`))
      (if (< (`/Game/Character/MainCharacter.CurrentPotionCount` _asmain_character) (`/Game/Character/MainCharacter.MaxPotionCount` _asmain_character))
        (if (<= (`self.CurrentStomach`) (`self.StomachSize`))
          (`KismetSystemLibrary.PrintString` "Got enough food")
          (`GameplayStatics.PlaySound2D` "/Game/MainLevel/FleshPit/WAV_Eat.WAV_Eat" 1.0 0.75 0.0 null null)
          (set `/Game/Character/MainCharacter.CurrentFoodUnits` (- (`/Game/Character/MainCharacter.CurrentFoodUnits` _asmain_character) (`self.FoodReqired`)) _asmain_character)
          (set `/Game/Character/MainCharacter.PitIsDigesting` true _asmain_character)
          (set `self.Eating` true)
          (`KismetSystemLibrary.PrintString` "He eat right now")
          (`KismetSystemLibrary.Delay` 1.0)
          (set `/Game/Character/MainCharacter.PitIsDigesting` false _asmain_character)
          (set `self.Eating` false)
          (`GameplayStatics.PlaySound2D` "/Game/MainLevel/FleshPit/WAV_Done.WAV_Done" 1.0 0.75 0.0 null null)
          (bind _output_get (set `/Game/Character/MainCharacter.CurrentPotionCount` (+ (`/Game/Character/MainCharacter.CurrentPotionCount` _asmain_character) 1) _asmain_character))
          (`KismetSystemLibrary.PrintString` "done digesting")
          (`KismetSystemLibrary.PrintString` (`KismetStringLibrary.Conv_IntToString` _output_get))
          (else
            (`KismetSystemLibrary.PrintString` "Eating too much")
            (goto _label)))
        (else
          (`KismetSystemLibrary.PrintString` "holding too many potions")
          (goto _label)))
      (else
        (`KismetSystemLibrary.PrintString` "You don't have enough food")
        (goto _label)))))

(fn `UserConstructionScript`)