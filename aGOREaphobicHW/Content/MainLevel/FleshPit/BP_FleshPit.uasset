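; Flesh pit actor that turns the first-person character's food units into potions on interaction.
; Entering its box shows a status widget for digesting, food or potion space, and enables input only when conversion is possible.
; A Gate lets Interact start a looped conversion until food or space runs out, then flags PitIsDigesting on the character.
; Leaving the box removes all widgets, disables input and closes the gate.
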(event `self.Box.OnComponentBeginOverlap`
  (params (OverlappedComponent :type "PrimitiveComponent Object Reference") (OtherActor :type "Actor Object Reference") (OtherComp :type "PrimitiveComponent Object Reference") (OtherBodyIndex :type Integer) (bFromSweep :type Boolean) (SweepResult :type "HitResult Structure (by ref)"))
  (bind _asbp_first_person_character (cast `/Game/FirstPerson/Blueprints/BP_FirstPersonCharacter` OtherActor))
  (if (`/Game/FirstPerson/Blueprints/BP_FirstPersonCharacter.PitIsDigesting` _asbp_first_person_character)
    (bind _returnvalue (`|CreateWidget` "/Game/MainLevel/FleshPit/WB_IsCurretlyEating.WB_IsCurretlyEating_C"))
    (`UserWidget.AddToViewport` _returnvalue 0)
    (`KismetSystemLibrary.PrintString` "Is currently eating")
    (elif (>= (`/Game/FirstPerson/Blueprints/BP_FirstPersonCharacter.CurrentFoodUnits` _asbp_first_person_character) (`self.FoodReqired`))
      (if (< (`/Game/FirstPerson/Blueprints/BP_FirstPersonCharacter.CurrentPotionCount` _asbp_first_person_character) (`/Game/FirstPerson/Blueprints/BP_FirstPersonCharacter.MaxPotionCount` _asbp_first_person_character))
        (bind _returnvalue_2 (`|CreateWidget` "/Game/MainLevel/FleshPit/WB_EnoughFood.WB_EnoughFood_C"))
        (`UserWidget.AddToViewport` _returnvalue_2 0)
        (`KismetSystemLibrary.PrintString` "got enough food")
        (`self.EnableInput` (`GameplayStatics.GetPlayerController` 0))
        (goto _label :!via `Open`)
        (else
          (bind _returnvalue_3 (`|CreateWidget` "/Game/MainLevel/FleshPit/WB_NotEnoughSpace.WB_NotEnoughSpace_C"))
          (`UserWidget.AddToViewport` _returnvalue_3 0)
          (`KismetSystemLibrary.PrintString` "Not enough Space")))
      (else
        (bind _returnvalue_4 (`|CreateWidget` "/Game/MainLevel/FleshPit/WB_NotEnoughFood.WB_NotEnoughFood_C"))
        (`UserWidget.AddToViewport` _returnvalue_4 0)
        (`KismetSystemLibrary.PrintString` "Not enough food")))))

(event `self.Box.OnComponentEndOverlap`
  (params (OverlappedComponent :type "PrimitiveComponent Object Reference") (OtherActor :type "Actor Object Reference") (OtherComp :type "PrimitiveComponent Object Reference") (OtherBodyIndex :type Integer))
  (`WidgetLayoutLibrary.RemoveAllWidgets`)
  (`self.DisableInput` (`GameplayStatics.GetPlayerController` 0))
  (goto _label :!via `Close`))

(event `InputAction|Interact`
  (params (Key :type "Key Structure"))
  (:`Pressed`
    (`/Engine/EditorBlueprintResources/StandardMacros.Gate` true :!label _label
      (:`Exit`
        (if (>= (`/Game/FirstPerson/Blueprints/BP_FirstPersonCharacter.CurrentFoodUnits` (stale `self.Box.OnComponentBeginOverlap` _asbp_first_person_character)) (`self.FoodReqired`)) :!label _label_2
          (if (< (`/Game/FirstPerson/Blueprints/BP_FirstPersonCharacter.CurrentPotionCount` (stale `self.Box.OnComponentBeginOverlap` _asbp_first_person_character)) (`/Game/FirstPerson/Blueprints/BP_FirstPersonCharacter.MaxPotionCount` (stale `self.Box.OnComponentBeginOverlap` _asbp_first_person_character)))
            (set `/Game/FirstPerson/Blueprints/BP_FirstPersonCharacter.CurrentFoodUnits` (- (`/Game/FirstPerson/Blueprints/BP_FirstPersonCharacter.CurrentFoodUnits` (stale `self.Box.OnComponentBeginOverlap` _asbp_first_person_character)) (`self.FoodReqired`)) (stale `self.Box.OnComponentBeginOverlap` _asbp_first_person_character))
            (set `/Game/FirstPerson/Blueprints/BP_FirstPersonCharacter.CurrentPotionCount` (+ (`/Game/FirstPerson/Blueprints/BP_FirstPersonCharacter.CurrentPotionCount` (stale `self.Box.OnComponentBeginOverlap` _asbp_first_person_character)) 1) (stale `self.Box.OnComponentBeginOverlap` _asbp_first_person_character))
            (`KismetSystemLibrary.PrintString` "1 potion made")
            (goto _label_2)
            (else
              _)))
        (set `/Game/FirstPerson/Blueprints/BP_FirstPersonCharacter.PitIsDigesting` true (stale `self.Box.OnComponentBeginOverlap` _asbp_first_person_character))))))

(fn `UserConstructionScript`)