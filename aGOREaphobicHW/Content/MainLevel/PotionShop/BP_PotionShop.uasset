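; Potion shop actor where the first-person player sells carried potions for money, limited to one sale until the market-visited flag clears.
; Entering the trigger box shows a widget for already visited, has potions, or no potions.
; With potions, it enables input and opens a gate so Interact adds potion value times count to Money, zeroes the count and sets WentToMarket.
; Leaving the box clears all widgets, disables input and closes the gate.
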(event `self.Box.OnComponentBeginOverlap`
  (params (OverlappedComponent :type "PrimitiveComponent Object Reference") (OtherActor :type "Actor Object Reference") (OtherComp :type "PrimitiveComponent Object Reference") (OtherBodyIndex :type Integer) (bFromSweep :type Boolean) (SweepResult :type "HitResult Structure (by ref)"))
  (bind _asbp_first_person_character (cast `/Game/FirstPerson/Blueprints/BP_FirstPersonCharacter` OtherActor))
  (if (`/Game/FirstPerson/Blueprints/BP_FirstPersonCharacter.WentToMarket` _asbp_first_person_character)
    (bind _returnvalue (`|CreateWidget` "/Game/MainLevel/PotionShop/WB_GoneToMarketAlready.WB_GoneToMarketAlready_C"))
    (`UserWidget.AddToViewport` _returnvalue 0)
    (`KismetSystemLibrary.PrintString` "Went to Market Today Already")
    (elif (> (`/Game/FirstPerson/Blueprints/BP_FirstPersonCharacter.CurrentPotionCount` _asbp_first_person_character) 0)
      (bind _returnvalue_2 (`|CreateWidget` "/Game/MainLevel/PotionShop/WB_GotPotions.WB_GotPotions_C"))
      (`UserWidget.AddToViewport` _returnvalue_2 0)
      (`KismetSystemLibrary.PrintString` "Got Potions")
      (`self.EnableInput` (`GameplayStatics.GetPlayerController` 0))
      (goto _label :!via `Open`)
      (else
        (bind _returnvalue_3 (`|CreateWidget` "/Game/MainLevel/PotionShop/WB_NoPotions.WB_NoPotions_C"))
        (`UserWidget.AddToViewport` _returnvalue_3 0)
        (`KismetSystemLibrary.PrintString` "No Potions")))))

(event `self.Box.OnComponentEndOverlap`
  (params (OverlappedComponent :type "PrimitiveComponent Object Reference") (OtherActor :type "Actor Object Reference") (OtherComp :type "PrimitiveComponent Object Reference") (OtherBodyIndex :type Integer))
  (`WidgetLayoutLibrary.RemoveAllWidgets`)
  (`self.DisableInput` (`GameplayStatics.GetPlayerController` 0))
  (goto _label :!via `Close`))

(event `InputAction|Interact`
  (params (Key :type "Key Structure"))
  (:`Pressed`
    (`/Engine/EditorBlueprintResources/StandardMacros.Gate` true :!label _label
      (:`Exit`
        (bind _output_get (set `self.TotalSellValue` (* (`self.PotionValue`) (`/Game/FirstPerson/Blueprints/BP_FirstPersonCharacter.CurrentPotionCount` (stale `self.Box.OnComponentBeginOverlap` _asbp_first_person_character)))))
        (`KismetSystemLibrary.PrintString` (`KismetStringLibrary.Conv_IntToString` _output_get))
        (set `/Game/FirstPerson/Blueprints/BP_FirstPersonCharacter.CurrentPotionCount` 0 (stale `self.Box.OnComponentBeginOverlap` _asbp_first_person_character))
        (bind _output_get_2 (set `/Game/FirstPerson/Blueprints/BP_FirstPersonCharacter.Money` (+ (`/Game/FirstPerson/Blueprints/BP_FirstPersonCharacter.Money` (stale `self.Box.OnComponentBeginOverlap` _asbp_first_person_character)) _output_get) (stale `self.Box.OnComponentBeginOverlap` _asbp_first_person_character)))
        (`KismetSystemLibrary.PrintString` (`KismetStringLibrary.Conv_IntToString` _output_get_2))
        (set `/Game/FirstPerson/Blueprints/BP_FirstPersonCharacter.WentToMarket` true (stale `self.Box.OnComponentBeginOverlap` _asbp_first_person_character))))))

(fn `UserConstructionScript`)